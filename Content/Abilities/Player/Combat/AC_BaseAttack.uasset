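; Base player attack component that drives a GravityPawn's melee or cast animation and attack state.
; PreAttack flags the owner as attacking, plays the first montage at its attack speed and spawns a fire emitter at the right-hand socket.
; Montage completion or interruption resets charged damage, removes the emitter and calls FinishAttacking, as does Attack directly.
; Hit is an empty stub; montage pause/resume logic is disconnected.
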(event Custom|PreAttack
  (bind _owner (Variables|Default|GetOwner))
  (bind _owner_2 (Variables|Default|GetOwner))
  (bind _owner_3 (Variables|Default|GetOwner))
  (bind _skeletalmesh (Variables|/Game/Pawns/GravityPawn.GravityPawn_C|GetSkeletalMesh _owner_2))
  (Variables|/Game/Pawns/GravityPawn.GravityPawn_C|SetAttacking _owner_2 true)
  (Animation|Montage|PlayMontage _skeletalmesh (Utilities|Array|Get(acopy) (Variables|Default|GetAnimation)) (Variables|/Game/Pawns/GravityPawn.GravityPawn_C|GetAttackSpeed _owner_2)
    (:then
      (bind _returnvalue (Effects|SpawnEmitteratLocation "/Game/StarterContent/Particles/P_Fire.P_Fire" (Transformation|GetSocketLocation _skeletalmesh "hand_r") "0, 0, 0" "0.500000,0.500000,0.500000" false)))
    (:OnCompleted
      (Variables|/Game/Pawns/GravityPawn.GravityPawn_C|SetAttacking _owner_3 false :!label _label)
      (Variables|/Game/Pawns/GravityPawn.GravityPawn_C|SetChargedDamage _owner (Math|Conversions|ToFloat(Integer) (Variables|/Game/Pawns/GravityPawn.GravityPawn_C|GetBaseDamage _owner)))
      (Components|DestroyComponent _returnvalue)
      (Default|FinishAttacking _owner_3))
    (:OnInterrupted
      (goto _label))))

(event Custom|Attack
  (Default|FinishAttacking (Variables|Default|GetOwner)))

(event EventBeginPlay
  (bind _asgravity_pawn (Utilities|Casting|CastToGravityPawn (Components|GetOwner)))
  (Variables|Default|SetOwner _asgravity_pawn))

(fn Hit)