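; Actor component for the player's stick melee attack, dealing charged damage to a struck pawn.
; Its Hit function sphere-traces for Pawn objects between the start and end melee sockets on the owner's skeletal mesh.
; On a hit, it applies the owner's ChargedDamage, truncated to a whole number, to that single traced actor.
; BeginPlay only calls the parent, and nothing in this graph calls Hit.
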(event EventBeginPlay
  (|CallParentFunction))

(fn Hit
  (bind _owner (Variables|Default|GetOwner))
  (bind _skeletalmesh (Variables|/Game/Pawns/GravityPawn.GravityPawn_C|GetSkeletalMesh _owner))
  (bind (_outhit _returnvalue) (Collision|SphereTraceForObjects (Transformation|GetSocketLocation _skeletalmesh "SocketMeleeStart") (Transformation|GetSocketLocation _skeletalmesh "SocketMeleeEnd") 1e+02 (Utilities|Array|MakeArray "ObjectTypeQuery3") false 0 "None"))
  (if _returnvalue
    (Game|Damage|ApplyDamage (.HitActor (Collision|BreakHitResult _outhit)) (Math|Conversions|ToFloat(Integer) (Math|Float|Truncate (Variables|/Game/Pawns/GravityPawn.GravityPawn_C|GetChargedDamage (Variables|Default|GetOwner)))) 0 0 "/Script/Engine.DamageType")))