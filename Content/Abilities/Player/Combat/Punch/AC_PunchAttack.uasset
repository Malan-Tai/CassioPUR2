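; AC_PunchAttack is a player combat component that deals the damage for a punch attack.
; Its Hit function runs a sphere overlap at the owner's right-hand socket, looking for Pawns other than the owner.
; Only the first actor found takes damage, using the owner's ChargedDamage value.
; The event graph holds no active logic, so Hit relies on an external caller.
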(event EventBeginPlay
  (|CallParentFunction) ; This node is disabled and will not be called.\nDrag off pins to build functionality.
)

(event EventTick
  (params (DeltaSeconds :type Float%20%28single-precision%29)))

(fn Hit
  (bind _outactors (Collision|SphereOverlapActors (Transformation|GetSocketLocation (Variables|/Game/Pawns/GravityPawn.GravityPawn_C|GetSkeletalMesh (Variables|Default|GetOwner)) "hand_R") 5e+01 (Utilities|Array|MakeArray "ObjectTypeQuery3") 0 (Utilities|Array|MakeArray (Variables|Default|GetOwner))))
  (if (Utilities|Array|IsValidIndex _outactors)
    (Game|Damage|ApplyDamage (Utilities|Array|Get(acopy) _outactors) (Variables|/Game/Pawns/GravityPawn.GravityPawn_C|GetChargedDamage (Variables|Default|GetOwner)) 0 0 "/Script/Engine.DamageType")))